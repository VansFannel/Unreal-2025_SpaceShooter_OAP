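; BP_SS_Pawn is the player pawn for the space shooter and handles movement from Enhanced Input.
; IA_Player_Move stores its value in InputMovement while triggered and zeroes it when completed or canceled.
; Tick offsets the actor along its right and forward vectors by that input, scaled by Speed and delta time for frame-rate independence.
; The move is set directly without sweep, so it does not stop on collisions.
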(event `self.ReceiveTick`
  (params (DeltaSeconds :type "Float (single-precision)"))
  (bind (_inputmovement_x _inputmovement_y) (`KismetMathLibrary.BreakVector2D` (`self.InputMovement`)))
  (bind _returnvalue (* DeltaSeconds (`self.Speed`)))
  ; Pawn's Movement
  (`self.K2_SetActorLocation` (+ (`self.K2_GetActorLocation`) (+ (* (`self.GetActorRightVector`) (* _inputmovement_x _returnvalue)) (* (* _inputmovement_y _returnvalue) (`self.GetActorForwardVector`))))))

(event `EnhancedInput|/Game/SpaceShooter/Input/Actions/IA_Player_Move`
  (params (ActionValue :type "Vector2D Structure") (ElapsedSeconds :type "Float (double-precision)") (TriggeredSeconds :type "Float (double-precision)") (InputAction :type "InputAction Object Reference" :default "/Game/SpaceShooter/Input/Actions/IA_Player_Move.IA_Player_Move"))
  (:`Triggered`
    (set `self.InputMovement` ActionValue))
  (:`Canceled`
    (set `self.InputMovement` (0.0 0.0) :!label _label))
  (:`Completed`
    (goto _label)))

(fn `UserConstructionScript`)