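; Player pawn for the space shooter, handling movement and firing through Enhanced Input.
; BeginPlay adds the default mapping context, and the move action drives movement input along the actor's forward and right vectors.
; The shoot action spawns a projectile at the FireSpawnPoint transform, then blocks firing until a timer re-enables it after FireDelay.
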(event `self.ReceiveBeginPlay`
  (bind _returnvalue (`GameplayStatics.GetPlayerController` 0))
  (`/Engine/EditorBlueprintResources/StandardMacros.IsValid` _returnvalue
    (:`Is Valid`
      (`EnhancedInputSubsystemInterface.AddMappingContext` (pcsubsystem `EnhancedInputLocalPlayerSubsystem` _returnvalue) "/Game/SpaceShooter/Input/IMC_Default.IMC_Default" 0 (struct)))))

(event `EnhancedInput|/Game/SpaceShooter/Input/Actions/IA_Player_Move`
  (params (ActionValue :type "Vector2D Structure") (ElapsedSeconds :type "Float (double-precision)") (TriggeredSeconds :type "Float (double-precision)") (InputAction :type "InputAction Object Reference" :default "/Game/SpaceShooter/Input/Actions/IA_Player_Move.IA_Player_Move"))
  ; Player's movement
  (:`Triggered`
    (`self.AddMovementInput` (`self.GetActorForwardVector`) ActionValue_Y)
    (`self.AddMovementInput` (`self.GetActorRightVector`) ActionValue_X)))

(event `EnhancedInput|/Game/SpaceShooter/Input/Actions/IA_Player_Shoot`
  (params (ActionValue :type Boolean) (ElapsedSeconds :type "Float (double-precision)") (TriggeredSeconds :type "Float (double-precision)") (InputAction :type "InputAction Object Reference" :default "/Game/SpaceShooter/Input/Actions/IA_Player_Shoot.IA_Player_Shoot"))
  ; Player's fire
  (:`Triggered`
    (if (`self.CanFire`)
      (`self.DoFire`)
      (set `self.CanFire` false)
      (`KismetSystemLibrary.K2_SetTimerDelegate` (delegate `EnableFire`) (`self.FireDelay`)))))

(event `EnableFire`
  ; Player's fire
  (set `self.CanFire` true))

(fn `DoFire`
  (`|SpawnActorFromClass` "/Game/SpaceShooter/Core/BP_SS_Projectile.BP_SS_Projectile_C" (`SceneComponent.K2_GetComponentToWorld` (`self.FireSpawnPoint`)) "Undefined" "MultiplyWithRoot" null null))

(fn `UserConstructionScript`)