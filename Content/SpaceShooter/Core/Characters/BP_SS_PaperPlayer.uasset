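; Player ship Blueprint for the space shooter, using a Paper2D flipbook sprite.
; The Enhanced Input move action feeds its Y and X values into movement input along the actor's forward and right vectors.
; UpdateAnimation picks a non-looping right or left ship flipbook from the X sign and prints the direction.
; Its only call and the other sprite animation logic in the event graph are disconnected, so the flipbook never changes at runtime.
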(event `self.ReceiveTick`
  (params (DeltaSeconds :type "Float (single-precision)")))

(event `EnhancedInput|/Game/SpaceShooter/Input/Actions/IA_Player_Move`
  (params (ActionValue :type "Vector2D Structure") (ElapsedSeconds :type "Float (double-precision)") (TriggeredSeconds :type "Float (double-precision)") (InputAction :type "InputAction Object Reference" :default "/Game/SpaceShooter/Input/Actions/IA_Player_Move.IA_Player_Move"))
  (:`Triggered`
    (`self.AddMovementInput` (`self.GetActorForwardVector`) ActionValue_Y)
    (`self.AddMovementInput` (`self.GetActorRightVector`) ActionValue_X)))

(event `self.Sprite.OnFinishedPlaying`)

(fn `UpdateAnimation`
  (params (ActionValueX :type "Float (double-precision)"))
  (`PaperFlipbookComponent.SetLooping` (`self.Sprite`) false)
  (if (> ActionValueX 0.0)
    (`PaperFlipbookComponent.SetFlipbook` (`self.Sprite`) "/Game/SpaceShooter/Art/Characters/SpaceShip/Flipbooks/PFB_SpaceShip_Right.PFB_SpaceShip_Right")
    (`KismetSystemLibrary.PrintString` "Right")
    (else
      (`PaperFlipbookComponent.SetFlipbook` (`self.Sprite`) "/Game/SpaceShooter/Art/Characters/SpaceShip/Flipbooks/PFB_SpaceShip_Left.PFB_SpaceShip_Left")
      (`KismetSystemLibrary.PrintString` "Left"))))

(fn `UserConstructionScript`)